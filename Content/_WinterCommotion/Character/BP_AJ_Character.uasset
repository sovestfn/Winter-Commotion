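; BP_AJ_Character is a player character with Enhanced Input jump and hold-to-run, starting at walk speed with gravity scale zeroed.
; When its health component reports death, it spawns a ceramic destruction effect, disables input, capsule collision and spring arm collision testing, then turns the mesh into a physics ragdoll.
; While dead, Tick moves the actor to the simulated mesh's location each frame.
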(event `self.ReceiveBeginPlay`
  (set `CharacterMovementComponent.MaxWalkSpeed` (`self.WalkSpeed`) (`self.CharacterMovement`))
  (set `CharacterMovementComponent.GravityScale` 0.0 (`self.CharacterMovement`))
  (`SceneComponent.K2_AddWorldRotation` :`self` (`self.Camera`)))

(event `EnhancedInput|/Game/_WinterCommotion/Core/Inputs/Actions/IA_Jump`
  (params (ActionValue :type Boolean) (ElapsedSeconds :type "Float (double-precision)") (TriggeredSeconds :type "Float (double-precision)") (InputAction :type "InputAction Object Reference" :default "/Game/_WinterCommotion/Core/Inputs/Actions/IA_Jump.IA_Jump"))
  (:`Triggered`
    (`self.Jump`))
  (:`Completed`
    (`self.StopJumping`)))

(event `EnhancedInput|/Game/_WinterCommotion/Core/Inputs/Actions/IA_Run`
  (params (ActionValue :type Boolean) (ElapsedSeconds :type "Float (double-precision)") (TriggeredSeconds :type "Float (double-precision)") (InputAction :type "InputAction Object Reference" :default "/Game/_WinterCommotion/Core/Inputs/Actions/IA_Run.IA_Run"))
  (:`Triggered`
    (set `CharacterMovementComponent.MaxWalkSpeed` (`self.RunSpeed`) (`self.CharacterMovement`)))
  (:`Completed`
    (set `CharacterMovementComponent.MaxWalkSpeed` (`self.WalkSpeed`) (`self.CharacterMovement`))))

(event `self.BP_HealthComponent.OnOwnerDied`
  (bind _mesh (`self.Mesh`))
  (set `self.bDead` true)
  (`GameplayStatics.SpawnEmitterAtLocation` "/Game/_WinterCommotion/VFX/Realistic_Starter_VFX_Pack_Vol2/Particles/Destruction/P_Destruction_Ceramic.P_Destruction_Ceramic" (`self.K2_GetActorLocation`))
  (`self.DisableInput` (`GameplayStatics.GetPlayerController` 0))
  (set `SpringArmComponent.bDoCollisionTest` false (`self.SpringArm`))
  (`PrimitiveComponent.SetCollisionEnabled` (`self.CapsuleComponent`) "NoCollision")
  (`PrimitiveComponent.SetCollisionEnabled` _mesh "QueryAndPhysics")
  (`PrimitiveComponent.SetSimulatePhysics` _mesh true)
  (`SkeletalMeshComponent.OverrideAnimationData` (`self.Mesh`) null false false 0.0 1.0))

(event `self.ReceiveTick`
  (params (DeltaSeconds :type "Float (single-precision)"))
  (if (`self.bDead`)
    (`self.K2_SetActorLocation` (`SceneComponent.K2_GetComponentLocation` (`self.Mesh`)))))

(fn `CurrentLevelName`
  (params (CurrentLevelName :type Name))
  (return))

(fn `UserConstructionScript`)