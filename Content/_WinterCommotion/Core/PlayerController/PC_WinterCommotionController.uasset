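; Player controller for WinterCommotion that handles the character's movement, look and pause input.
; On BeginPlay it loads look sensitivity from the game instance's saved settings, adds the Enhanced Input mapping context and caches the pawn's movement component.
; Movement feeds that component along control-rotation axes, while look input is scaled by sensitivity.
; Pause toggles the game pause, a reused menu widget, input mode and cursor; SetSettings is an empty stub.
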(event `self.ReceiveBeginPlay`
  (`|ExecutionSequence`
    (:`then_0`
      (bind _asgi_winter_commotion (cast `/Game/_WinterCommotion/Core/GameInstances/GI_WinterCommotion` (`GameplayStatics.GetGameInstance`)))
      (bind _s_savesettings_sensetivity (break `/Game/_WinterCommotion/Core/Structures/S_GameSettings` (`/Game/_WinterCommotion/Core/GameInstances/GI_WinterCommotion.S_SaveSettings` _asgi_winter_commotion)))
      (set `self.Sensetivity Value` _s_savesettings_sensetivity))
    (:`then_1`
      (`WidgetBlueprintLibrary.SetInputMode_GameOnly` self)
      (set `self.bShowMouseCursor` false)
      (`EnhancedInputSubsystemInterface.AddMappingContext` (subsystem `EnhancedInputLocalPlayerSubsystem`) "/Game/_WinterCommotion/Core/Inputs/IMC_Character.IMC_Character" 0 (struct))
      (bind _asbp_aj_character (cast `/Game/_WinterCommotion/Character/BP_AJ_Character` (`self.K2_GetPawn`)))
      (bind _output_get (set `self.BP_AJCharacter` _asbp_aj_character))
      (set `self.Character MovementComp` (`Character.CharacterMovement` _output_get)))))

(event `EnhancedInput|/Game/_WinterCommotion/Core/Inputs/Actions/IA_Movement`
  (params (ActionValue :type "Vector2D Structure") (ElapsedSeconds :type "Float (double-precision)") (TriggeredSeconds :type "Float (double-precision)") (InputAction :type "InputAction Object Reference" :default "/Game/_WinterCommotion/Core/Inputs/Actions/IA_Movement.IA_Movement"))
  (:`Triggered`
    (`self.MoveCalculate` ActionValue_X ActionValue_Y)))

(event `EnhancedInput|/Game/_WinterCommotion/Core/Inputs/Actions/IA_Looking`
  (params (ActionValue :type "Vector2D Structure") (ElapsedSeconds :type "Float (double-precision)") (TriggeredSeconds :type "Float (double-precision)") (InputAction :type "InputAction Object Reference" :default "/Game/_WinterCommotion/Core/Inputs/Actions/IA_Looking.IA_Looking"))
  (:`Triggered`
    (`self.AddYawInput` (* ActionValue_X (`self.Sensetivity Value`)))
    (`self.AddPitchInput` (* ActionValue_Y (`self.Sensetivity Value`)))))

(event `EnhancedInput|/Game/_WinterCommotion/Core/Inputs/Actions/IA_PauseMenu`
  (params (ActionValue :type Boolean) (ElapsedSeconds :type "Float (double-precision)") (TriggeredSeconds :type "Float (double-precision)") (InputAction :type "InputAction Object Reference" :default "/Game/_WinterCommotion/Core/Inputs/Actions/IA_PauseMenu.IA_PauseMenu"))
  (:`Triggered`
    (if (`GameplayStatics.IsGamePaused`)
      (`GameplayStatics.SetGamePaused` false)
      (`WidgetBlueprintLibrary.SetInputMode_GameOnly` self)
      (set `self.bShowMouseCursor` false)
      (bind _wbp_pausemenu (`self.WBP_PauseMenu`)
        (:`then`
          (`Widget.RemoveFromParent` _wbp_pausemenu))
        (:`else`))
      (else
        (`GameplayStatics.SetGamePaused` true)
        (`self.WBP_PauseMenu`
          (:`then`
            _)
          (:`else`
            (bind _returnvalue (`|CreateWidget` "/Game/_WinterCommotion/UI/WBP_PauseMenu.WBP_PauseMenu_C" self))
            (bind _output_get (set `self.WBP_PauseMenu` _returnvalue))))
        (`UserWidget.AddToViewport` _output_get 0)
        (`WidgetBlueprintLibrary.SetInputMode_GameAndUIEx` self _output_get)
        (set `self.bShowMouseCursor` true)))))

(fn `MoveCalculate`
  (params (B :type "Float (double-precision)") (B2 :type "Float (double-precision)"))
  (bind (_returnvalue_roll _returnvalue_pitch _returnvalue_yaw) (`KismetMathLibrary.BreakRotator` (`self.GetControlRotation`)))
  (bind (_returnvalue_roll_2 _returnvalue_pitch_2 _returnvalue_yaw_2) (`KismetMathLibrary.BreakRotator` (`self.GetControlRotation`)))
  (bind _character_movementcomp (`self.Character MovementComp`)
    (:`then`
      (`|ExecutionSequence`
        (:`then_0`
          (`PawnMovementComponent.AddInputVector` _character_movementcomp (* (`KismetMathLibrary.GetForwardVector` (`KismetMathLibrary.MakeRotator` 0.0 0.0 _returnvalue_yaw)) B2) false))
        (:`then_1`
          (`PawnMovementComponent.AddInputVector` _character_movementcomp (* (`KismetMathLibrary.GetRightVector` (`KismetMathLibrary.MakeRotator` _returnvalue_roll_2 0.0 _returnvalue_yaw_2)) B) false))))
    (:`else`)))

(fn `SetSettings`
  (returns (S_GameSettings :type "/Game/_WinterCommotion/Core/Structures/S_GameSettings Structure"))
  (return))

(fn `UserConstructionScript`)