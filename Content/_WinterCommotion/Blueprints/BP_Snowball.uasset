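; BP_Snowball is a projectile that damages actors tagged Player on impact.
; Tick moves it along its forward vector with a swept offset, and the bound hit event spawns ice particles and a target-specific sound, then destroys it.
; BeginPlay also caches the game instance and plays a launch sound; a TurnToPlayer function, not called here, can aim it at the first player's pawn.
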(event `self.ReceiveBeginPlay`
  (`|ExecutionSequence`
    (:`then_0`
      (`self.Binds`))
    (:`then_1`
      (`self.Casts`))
    (:`then_2`
      (`GameplayStatics.SpawnSoundAtLocation` "/Game/_WinterCommotion/Sounds/Props/snowball_sound_start.snowball_sound_start" (`self.K2_GetActorLocation`) (struct) 1.0 1.0 0.0 null null))))

(event `self.ReceiveTick`
  (params (DeltaSeconds :type "Float (single-precision)"))
  (`self.K2_AddActorWorldOffset` (* (* DeltaSeconds (`self.Speed`)) (`self.GetActorForwardVector`)) true))

(event `OnActorHit_Event`
  (params (SelfActor :type "Actor Object Reference") (OtherActor :type "Actor Object Reference") (NormalImpulse :type "Vector Structure") (Hit :type "HitResult Structure (by ref)"))
  (bind _returnvalue (`self.K2_GetActorLocation`))
  (`/Engine/EditorBlueprintResources/StandardMacros.IsValid` OtherActor
    (:`Is Valid`
      (if (`self.ActorHasTag` OtherActor "Player")
        (`GameplayStatics.ApplyDamage` OtherActor (`self.Base Damage`) null self)
        (`GameplayStatics.SpawnEmitterAtLocation` "/Game/_WinterCommotion/VFX/Realistic_Starter_VFX_Pack_Vol2/Particles/Hit/P_Ice.P_Ice" _returnvalue)
        (`GameplayStatics.SpawnSoundAtLocation` "/Game/_WinterCommotion/Sounds/Props/Mgc_Ice_Arrow_Hit_01_Cue.Mgc_Ice_Arrow_Hit_01_Cue" _returnvalue (struct) 1.0 1.0 0.0 null null)
        (else
          (`GameplayStatics.SpawnEmitterAtLocation` "/Game/_WinterCommotion/VFX/Realistic_Starter_VFX_Pack_Vol2/Particles/Hit/P_Ice.P_Ice" _returnvalue)
          (`GameplayStatics.SpawnSoundAtLocation` "/Game/_WinterCommotion/Sounds/Props/snowball_sound.snowball_sound" _returnvalue (struct) 1.0 1.0 0.0 null null)))
      (`self.K2_DestroyActor`))))

(fn `Binds`
  (add `self.OnActorHit` (`|CreateDelegate` :!event `OnActorHit_Event`)))

(fn `Casts`
  (bind _asgi_winter_commotion (cast `/Game/_WinterCommotion/Core/GameInstances/GI_WinterCommotion` (`GameplayStatics.GetGameInstance`)))
  (set `self.GI_WinterCommotion` _asgi_winter_commotion))

(fn `UserConstructionScript`)