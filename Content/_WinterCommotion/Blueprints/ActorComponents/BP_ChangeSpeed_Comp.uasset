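; Actor component that scales the player character's walk and run speeds by a coefficient.
; On BeginPlay it caches player 0's BP_AJ_Character pawn and its default run and walk speeds.
; ChangeSpeed multiplies those cached defaults by SpeedCoeff, so repeated calls do not stack, and SetDefaultSpeed restores them.
; Both set MaxWalkSpeed from the walk speed; SetSpeedCoeff only stores the value without applying it.
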(event `self.ReceiveBeginPlay`
  (bind _asbp_aj_character (cast `/Game/_WinterCommotion/Character/BP_AJ_Character` (`GameplayStatics.GetPlayerPawn` 0)))
  (`/Engine/EditorBlueprintResources/StandardMacros.IsValid` _asbp_aj_character
    (:`Is Valid`
      (bind _output_get (set `self.BP_AJCharacter` _asbp_aj_character))
      (set `self.DefaultRunSpeed` (`/Game/_WinterCommotion/Character/BP_AJ_Character.RunSpeed` _output_get))
      (set `self.DefaultWalkSpeed` (`/Game/_WinterCommotion/Character/BP_AJ_Character.WalkSpeed` _output_get)))))

(fn `ChangeSpeed`
  (bind _bp_ajcharacter (`self.BP_AJCharacter`))
  (bind _returnvalue (* (`self.DefaultWalkSpeed`) (`self.SpeedCoeff`)))
  (set `/Game/_WinterCommotion/Character/BP_AJ_Character.RunSpeed` (* (`self.DefaultRunSpeed`) (`self.SpeedCoeff`)) _bp_ajcharacter)
  (set `/Game/_WinterCommotion/Character/BP_AJ_Character.WalkSpeed` _returnvalue _bp_ajcharacter)
  (set `CharacterMovementComponent.MaxWalkSpeed` _returnvalue (`Character.CharacterMovement` _bp_ajcharacter)))

(fn `GetSpeedCoeff`
  (returns (SpeedCoeff :type "Float (single-precision)"))
  (return (`self.SpeedCoeff`)))

(fn `SetDefaultSpeed`
  (bind _bp_ajcharacter (`self.BP_AJCharacter`))
  (bind _defaultwalkspeed (`self.DefaultWalkSpeed`))
  (set `/Game/_WinterCommotion/Character/BP_AJ_Character.RunSpeed` (`self.DefaultRunSpeed`) _bp_ajcharacter)
  (set `/Game/_WinterCommotion/Character/BP_AJ_Character.WalkSpeed` _defaultwalkspeed _bp_ajcharacter)
  (set `CharacterMovementComponent.MaxWalkSpeed` _defaultwalkspeed (`Character.CharacterMovement` _bp_ajcharacter)))

(fn `SetSpeedCoeff`
  (params (SpeedCoeff :type "Float (single-precision)"))
  (set `self.SpeedCoeff` SpeedCoeff))