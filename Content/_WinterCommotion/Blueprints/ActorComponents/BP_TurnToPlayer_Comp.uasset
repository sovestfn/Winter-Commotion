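; Actor component that turns its owning actor to face the first player's pawn once, when play begins.
; TurnToPlayer builds a rotation from the normalized direction toward the pawn, zeroes pitch so the owner stays level, and applies it to the owner.
; It does nothing if the player pawn is not valid, and there is no tick update to keep tracking the player.
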(event `self.ReceiveBeginPlay`
  (`self.TurnToPlayer`))

(fn `TurnToPlayer`
  (bind _returnvalue (`GameplayStatics.GetPlayerPawn` 0))
  (bind _returnvalue_2 (`self.GetOwner`))
  (`/Engine/EditorBlueprintResources/StandardMacros.IsValid` _returnvalue
    (:`Is Valid`
      (`Actor.K2_SetActorRotation` _returnvalue_2 (`KismetMathLibrary.MakeRotator` (.roll (`KismetMathLibrary.MakeRotFromX` (`KismetMathLibrary.Normal` (- (`Actor.K2_GetActorLocation` _returnvalue) (`Actor.K2_GetActorLocation` _returnvalue_2))))) 0.0 (.yaw (`KismetMathLibrary.MakeRotFromX` (`KismetMathLibrary.Normal` (- (`Actor.K2_GetActorLocation` _returnvalue) (`Actor.K2_GetActorLocation` _returnvalue_2)))))) false))))