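; Actor component that spawns BP_Snowball actors for its owner in Winter Commotion, with damage scaled by game difficulty.
; On BeginPlay it caches the game instance and game state, then picks base damage from the difficulty setting.
; SpawnBallEvent spawns a snowball at the owner's SphereComponent location and passes it that damage.
; Snowball counting on the game state is an unused placeholder, and the spawn dispatcher binding is disconnected.
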(event `self.ReceiveBeginPlay`
  (`|ExecutionSequence`
    (:`then_0`
      (`self.Casts`))
    (:`then_2`
      (`self.GetBallDamageVar`))))

(event `SpawnBallEvent`
  (`self.SpawnBall`))

(fn `Binds`)

(fn `Casts`
  (`|ExecutionSequence`
    (:`then_0`
      (bind _asgi_winter_commotion (cast `/Game/_WinterCommotion/Core/GameInstances/GI_WinterCommotion` (`GameplayStatics.GetGameInstance`)))
      (set `self.GI_WinterCommotion` _asgi_winter_commotion))
    (:`then_1`
      (bind _asgs_winter_commotion (cast `/Game/_WinterCommotion/Core/GameStates/GS_WinterCommotion` (`GameplayStatics.GetGameState`)))
      (set `self.GS_WinterCommotion` _asgs_winter_commotion))))

(fn `GetBallDamageVar`
  (set `self.BaseBallDamage` (select `/Game/_WinterCommotion/Core/Enums/ENUM_GameDifficulty` (`/Game/_WinterCommotion/Core/GameInstances/GI_WinterCommotion.Get_GameDifficulty` (`self.GI_WinterCommotion`)) :`NewEnumerator0` 25.0 :`NewEnumerator1` 50.0 :`NewEnumerator2` 90.0)))

(fn `SpawnBall`
  (bind _returnvalue (`Actor.GetComponentByClass` (`self.GetOwner`) "/Script/Engine.SphereComponent"))
  (`/Engine/EditorBlueprintResources/StandardMacros.IsValid` _returnvalue
    (:`Is Valid`
      (`|SpawnActorFromClass` "/Game/_WinterCommotion/Blueprints/BP_Snowball.BP_Snowball_C" (`KismetMathLibrary.Conv_VectorToTransform` (`SceneComponent.K2_GetComponentLocation` _returnvalue)) "AdjustIfPossibleButAlwaysSpawn" "MultiplyWithRoot" null (`self.BaseBallDamage`) null))))

(fn `SpawnedCount`
  ;[1 1 1] Пока не используется - на случай, если понадобится считать снежки
  (bind _gs_wintercommotion (`self.GS_WinterCommotion`)
    (:`then`
      (`/Engine/EditorBlueprintResources/StandardMacros.IncrementInt` (`/Game/_WinterCommotion/Core/GameStates/GS_WinterCommotion.Get_SnowBallsCount` _gs_wintercommotion)
        (:`  `
          (`/Game/_WinterCommotion/Core/GameStates/GS_WinterCommotion.Set_SnowBallsCount` _gs_wintercommotion 0))))
    (:`else`)))