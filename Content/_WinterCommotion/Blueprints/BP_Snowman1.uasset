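; BP_Snowman1 is a snowman actor that faces the player and spawns balls while the player is nearby.
; Player overlap spawns a ball through BPSpawnerComponent and starts a looping timer, which is cleared when overlap ends.
; Tick delegates turning to BPTurnToPlayerComponent, though the Blueprint also holds its own TurnToPlayer graph with zeroed pitch.
; Construction randomizes the look by giving each listed material a weighted chance to override the first slot.
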(event `self.ReceiveActorBeginOverlap`
  (params (OtherActor :type "Actor Object Reference"))
  (if (`self.ActorHasTag` OtherActor "Player")
    (bind _returnvalue (`KismetSystemLibrary.K2_SetTimerDelegate` (`|CreateDelegate` (`self.BP_SpawnerComponent`) :!event `SpawnBall`) 2.0 true))
    (set `self.SpawnTimerHandler` _returnvalue)
    (`/Game/_WinterCommotion/Blueprints/ActorComponents/BP_SnowballSpawner_Comp.SpawnBall` (`self.BP_SpawnerComponent`))))

(event `self.ReceiveActorEndOverlap`
  (params (OtherActor :type "Actor Object Reference"))
  (if (`self.ActorHasTag` OtherActor "Player")
    (`KismetSystemLibrary.K2_ClearAndInvalidateTimerHandle` (`self.SpawnTimerHandler`))))

(event `self.ReceiveTick`
  (params (DeltaSeconds :type "Float (single-precision)"))
  (`/Game/_WinterCommotion/Blueprints/ActorComponents/BP_TurnToPlayer_Comp.TurnToPlayer` (`self.BP_TurnToPlayerComponent`)))

(fn `Casts`
  (`|ExecutionSequence`
    (:`then_0`
      (cast `/Game/_WinterCommotion/Core/GameStates/GS_WinterCommotion` (`GameplayStatics.GetGameState`)))
    (:`then_1`
      (cast `/Game/_WinterCommotion/Core/GameMods/GM_Arcade` (`GameplayStatics.GetGameMode`)))))

(fn `UserConstructionScript`
  (locals (SnowmanMaterials :type "Array of MaterialInstance Object Reference"))
  (for _array_element (`self.MaterialSnowman`)
    (if (`KismetMathLibrary.RandomBoolWithWeight` 0.3)
      (`PrimitiveComponent.SetMaterial` (`self.Snowman`) 0 _array_element))))