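; Gift box pickable for Winter Commotion that adds a point to the first player's score whenever it is destroyed.
; BeginPlay caches that player's PS_WinterCommotion player state and assigns the bonus sound and destruction effect variables.
; The construction script randomizes the ribbon by giving each listed material a 20% chance to apply to two meshes, so later hits override earlier ones.
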(event `self.ReceiveBeginPlay`
  (`|ExecutionSequence`
    (:`then_0`
      (`self.Casts`))
    (:`then_1`
      (set `self.Sound` "/Game/_WinterCommotion/Sounds/Props/bonus_Cue.bonus_Cue")
      (set `self.DestroyEffect` "/Game/_WinterCommotion/VFX/Realistic_Starter_VFX_Pack_Vol2/Particles/Destruction/P_Destruction_Metal.P_Destruction_Metal"))))

(event `self.ReceiveDestroyed`
  (bind _ps_wintercommotion (`self.PS_WinterCommotion`)
    (:`then`
      (bind _result (`/Engine/EditorBlueprintResources/StandardMacros.IncrementInt` (`/Game/_WinterCommotion/Core/PlayerStates/PS_WinterCommotion.Get_CurrentScore` _ps_wintercommotion))
        (:`  `
          (`/Game/_WinterCommotion/Core/PlayerStates/PS_WinterCommotion.Set_CurrentScore` _ps_wintercommotion _result))))
    (:`else`)))

(fn `Casts`
  (bind _asps_winter_commotion (cast `/Game/_WinterCommotion/Core/PlayerStates/PS_WinterCommotion` (`GameplayStatics.GetPlayerState` 0)))
  (set `self.PS_WinterCommotion` _asps_winter_commotion))

(fn `Set_RandomColorForRibbon`
  (for _array_element (`self.MaterialRibbon`)
    (if (`KismetMathLibrary.RandomBoolWithWeight` 0.2)
      (`|ExecutionSequence`
        (:`then_0`
          (`PrimitiveComponent.SetMaterial` (`self.giftbox_fbx_Giftbox02`) 0 _array_element))
        (:`then_1`
          (`PrimitiveComponent.SetMaterial` (`self.giftbox_fbx_Giftbox03`) 0 _array_element))))))

(fn `UserConstructionScript`
  (`self.Set_RandomColorForRibbon`))