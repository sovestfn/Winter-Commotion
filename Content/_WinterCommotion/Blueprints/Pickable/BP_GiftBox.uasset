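; BP_GiftBox is a pickable gift that adds one point to the player's score whenever it is destroyed.
; BeginPlay caches player 0's PS_WinterCommotion and sets the bonus sound; Destroyed increments that state's score.
; The construction script randomizes box, ribbon and bow materials from a shared array.
; Each entry gets a coin flip and the last success wins, favoring later entries or leaving the default.
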(event `self.ReceiveBeginPlay`
  (`|ExecutionSequence`
    (:`then_0`
      (`self.Casts`))
    (:`then_1`
      (set `self.Sound` "/Game/_WinterCommotion/Sounds/Props/bonus_Cue.bonus_Cue"))))

(event `self.ReceiveDestroyed`
  (bind _ps_wintercommotion (`self.PS_WinterCommotion`)
    (:`then`
      (bind _result (`/Engine/EditorBlueprintResources/StandardMacros.IncrementInt` (`/Game/_WinterCommotion/Core/PlayerStates/PS_WinterCommotion.Get_PlayerScore` _ps_wintercommotion))
        (:`  `
          (`/Game/_WinterCommotion/Core/PlayerStates/PS_WinterCommotion.Set_PlayerScore` _ps_wintercommotion _result))))
    (:`else`)))

(fn `Casts`
  (bind _asps_winter_commotion (cast `/Game/_WinterCommotion/Core/PlayerStates/PS_WinterCommotion` (`GameplayStatics.GetPlayerState` 0)))
  (set `self.PS_WinterCommotion` _asps_winter_commotion))

(fn `RandomColorForBow`
  (for _array_element (`self.MaterialGiftBox`)
    (if (`KismetMathLibrary.RandomBoolWithWeight` 0.5)
      (`PrimitiveComponent.SetMaterial` (`self.giftbox_fbx_Giftbox01`) 0 _array_element))))

(fn `RandomColorForBox`
  (for _array_element (`self.MaterialGiftBox`)
    (if (`KismetMathLibrary.RandomBoolWithWeight` 0.5)
      (`PrimitiveComponent.SetMaterial` (`self.giftbox_fbx_Giftbox03`) 0 _array_element))))

(fn `RandomColorForRibbon`
  (for _array_element (`self.MaterialGiftBox`)
    (if (`KismetMathLibrary.RandomBoolWithWeight` 0.5)
      (`PrimitiveComponent.SetMaterial` (`self.giftbox_fbx_Giftbox02`) 0 _array_element))))

(fn `UserConstructionScript`
  (`|ExecutionSequence`
    (:`then_0`
      (`self.RandomColorForBox`))
    (:`then_1`
      (`self.RandomColorForRibbon`))
    (:`then_2`
      (`self.RandomColorForBow`))))