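; BP_Bonus is a bonus actor that reacts when an actor tagged "Player" begins or ends overlapping it.
; Each overlap either sets a one-shot timer from StartDelay or EndDelay, or calls StartBonusEvent or EndBonusEvent immediately when that delay is not positive.
; Both bonus events only clear their own timer handle and apply no effect here, so the Blueprint reads as a base for specific bonuses.
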(event `self.ReceiveActorBeginOverlap`
  (params (OtherActor :type "Actor Object Reference"))
  (`/Engine/EditorBlueprintResources/StandardMacros.IsValid` OtherActor
    (:`Is Valid`
      (if (`self.ActorHasTag` OtherActor "Player")
        (if (> (`self.StartDelay`) 0.0)
          (bind _returnvalue (`KismetSystemLibrary.K2_SetTimerDelegate` (`|CreateDelegate` :!event `StartBonusEvent`) (`self.StartDelay`)))
          (set `self.StartHandler` _returnvalue)
          (else
            (`self.StartBonusEvent`)))))))

(event `self.ReceiveActorEndOverlap`
  (params (OtherActor :type "Actor Object Reference"))
  (`/Engine/EditorBlueprintResources/StandardMacros.IsValid` OtherActor
    (:`Is Valid`
      (if (`self.ActorHasTag` OtherActor "Player")
        (if (> (`self.EndDelay`) 0.0)
          (bind _returnvalue (`KismetSystemLibrary.K2_SetTimerDelegate` (`|CreateDelegate` :!event `EndBonusEvent`) (`self.EndDelay`)))
          (set `self.EndHandler` _returnvalue)
          (else
            (`self.EndBonusEvent`)))))))

(event `EndBonusEvent`
  (bind _endhandler (`self.EndHandler`))
  (if (`KismetSystemLibrary.K2_IsValidTimerHandle` _endhandler)
    (`KismetSystemLibrary.K2_ClearAndInvalidateTimerHandle` _endhandler)))

(event `StartBonusEvent`
  (bind _starthandler (`self.StartHandler`))
  (if (`KismetSystemLibrary.K2_IsValidTimerHandle` _starthandler)
    (`KismetSystemLibrary.K2_ClearAndInvalidateTimerHandle` _starthandler)))

(fn `UserConstructionScript`)